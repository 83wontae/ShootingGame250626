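; Player controller for the shooting game mode that hands the player's nickname from the game instance to the player state on possession.
; Possess triggers ResClientPossess, which prints a debug string and reads NickName from BP_GameInstance.
; It passes the name through ReqChangeNickName to ChangeNickName on BP_ShootingPlayerState.
; The Res and Req event names suggest a client-response and server-request round trip.
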(event Custom|ResClientPossess
  (Development|PrintString "ResClientPossess" true true "(R=0.000000,G=0.660000,B=1.000000,A=1.000000)" 6e+01)
  (bind _asbp_game_instance (Utilities|Casting|CastToBP_GameInstance (Game|GetGameInstance)))
  (CallFunction|ReqChangeNickName (Variables|/Game/Shooting/GameMode/BP_GameInstance.BP_GameInstance_C|GetNickName _asbp_game_instance)))

(event Custom|ReqChangeNickName
  (params (NickName :type String))
  (bind _asbp_shooting_player_state (Utilities|Casting|CastToBP_ShootingPlayerState (Variables|GetPlayerState)))
  (Default|ChangeNickName _asbp_shooting_player_state NickName))

(event EventPossess
  (params (PossessedPawn :type Pawn%20Object%20Reference))
  (CallFunction|ResClientPossess))

(fn ConstructionScript)