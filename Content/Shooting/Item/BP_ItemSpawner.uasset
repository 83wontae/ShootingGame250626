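; Item spawner that keeps one random item from its Items list spawned at its own transform, starting at BeginPlay.
; DoRandomItemSpawn runs only on authority, destroying the previous item, spawning a new one and binding to its destruction.
; A function-name timer re-runs the spawn to swap the item after a random delay, or retry after a failed spawn.
; EventItemDestroy resets that timer to a fixed respawn delay.
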(event EventBeginPlay
  (CallFunction|DoRandomItemSpawn))

(fn ConstructionScript)

(fn DoRandomItemSpawn
  (Networking|SwitchHasAuthority
    (:Authority
      (bind _spawnitem (Variables|Default|GetSpawnItem)
        (:then
          (Actor|DestroyActor _spawnitem))
        (:else
          _))
      (bind _returnvalue (Game|SpawnActorfromClass (.OutItem (Utilities|Array|Random (Variables|Default|GetItems))) (Transformation|GetActorTransform) "Undefined" "MultiplyWithRoot" 0 0))
      (bind _output_get (Variables|Default|SetSpawnItem _returnvalue))
      (Utilities|IsValid _output_get
        (:Is%20Valid
          (Game|BindEventtoOnDestroyed _output_get (EventDispatchers|CreateEvent :!event EventItemDestroy))
          (Utilities|Time|SetTimerbyFunctionName 0 "DoRandomItemSpawn" (Math|Random|RandomFloatinRange 5.0 1e+01)))
        (:Is%20Not%20Valid
          (Utilities|Time|SetTimerbyFunctionName 0 "DoRandomItemSpawn" 5.0))))))

(fn EventItemDestroy
  (params (DestroyedActor :type Actor%20Object%20Reference))
  (Utilities|Time|ClearTimerbyFunctionName 0 "DoRandomItemSpawn")
  (Utilities|Time|SetTimerbyFunctionName 0 "DoRandomItemSpawn" 5.0))