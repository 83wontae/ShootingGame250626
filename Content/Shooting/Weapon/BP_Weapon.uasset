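; Networked hitscan weapon, configured by WeaponData, that attaches to a character's weapon socket and simulates physics when dropped.
; Trigger and reload play montages; separate fire and reload-complete events spawn muzzle effects and send server requests from the local player.
; The server line-traces from the client's camera ray, applies damage, and refills ammo using PlayerState magazines.
; Buffs can override ammo checks, and Ammo's OnRep updates the owner's HUD.
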(event Custom|ReqFire
  (params (StartLoc :type Vector) (EndLoc :type Vector))
  ;[0.15 0 0 0.5] Server
  (bind _isused (CallFunction|UseAmmo))
  (if _isused
    (bind _outhit (Collision|LineTraceForObjects StartLoc EndLoc (Utilities|Array|MakeArray "ObjectTypeQuery1" "ObjectTypeQuery2" "ObjectTypeQuery3" "ObjectTypeQuery4" "ObjectTypeQuery5" "ObjectTypeQuery6") false (Utilities|Array|MakeArray (Variables|Default|GetCharacter)) "ForDuration" true "(R=1.000000,G=0.000000,B=0.000000,A=1.000000)" "(R=0.000000,G=1.000000,B=0.000000,A=1.000000)" 1e+01))
    (Game|Damage|ApplyDamage (.HitActor (Collision|BreakHitResult _outhit)) (.damage (Variables|Default|GetWeaponData)) (Pawn|GetController (Variables|Default|GetCharacter)) self)))

(event Custom|ReqReload
  ;[0.15 0 0 0.5] (Server) Reload
  (bind _character (Variables|Default|GetCharacter)
    (:then
      (bind _asbp_shooting_player_state (Utilities|Casting|CastToBP_ShootingPlayerState (Variables|/Script/Engine.Pawn|GetPlayerState _character)))
      (bind _isused (Default|UseMag _asbp_shooting_player_state))
      (if _isused
        (Variables|Default|SetAmmo (.maxammo (Variables|Default|GetWeaponData)))))
    (:else)))

(event EventBeginPlay
  (bind _weapondata (Variables|Default|GetWeaponData))
  (Variables|Default|SetAmmo (.maxammo _weapondata))
  (Components|StaticMesh|SetStaticMesh (Variables|Default|GetWeapon) (.weaponmesh _weapondata)))

(fn ConstructionScript)

(fn DoTrigger
  (bind _character (Variables|Default|GetCharacter)
    (:then
      (Animation|PlayAnimMontage _character (.shootmontage (Variables|Default|GetWeaponData)) 1.0 "None"))
    (:else)))

(fn DoFireEffect
  (bind _weapon (Variables|Default|GetWeapon))
  (bind _returnvalue (Transformation|GetSocketTransform _weapon "muzzle" "RTS_World"))
  (Effects|SpawnEmitteratLocation "/Game/StarterContent/Particles/P_Explosion.P_Explosion" (.location _returnvalue) (.rotation _returnvalue) "0.100000,0.100000,0.100000")
  (Audio|SpawnSoundatLocation "/Game/StarterContent/Audio/Explosion_Cue.Explosion_Cue" (.location _returnvalue) "0, 0, 0" 1.0 1.0 0.0 0 0))

(fn HasOwner
  (return (Utilities|IsValid (Variables|Default|GetCharacter))))

(fn EventMontageEnd
  (params (Montage :type Anim%20Montage%20Object%20Reference) (bInterrupted :type Boolean)))

(fn UseAmmo
  ;[0.15 0 0 0.5] (Server)
  (if (CallFunction|CanShoot)
    (Variables|Default|SetAmmo (Math|Integer|Clamp(Integer) (- (Variables|Default|GetAmmo) 1) 0 (.maxammo (Variables|Default|GetWeaponData))))
    (return true)
    (else
      (return false))))

(fn UpdateAmmoUI
  (params (Ammo :type Integer))
  (if (== (Variables|Default|GetCharacter) (Pawn|GetControlledPawn (Game|GetPlayerController 0)))
    (bind _asbp_shooting_hud (Utilities|Casting|CastToBP_ShootingHud (HUD|GetHUD (Game|GetPlayerController 0))))
    (Default|UpdateAmmo _asbp_shooting_hud Ammo)))

(fn OnRepAmmo
  ;[0.15 0.15 0.15 0.5] Client
  (CallFunction|UpdateAmmoUI (Variables|Default|GetAmmo)))

(fn CanShoot
  (bind _character (Variables|Default|GetCharacter))
  (bind _returnvalue (Actor|GetComponentbyClass _character "/Game/Shooting/Buff/BP_BuffComponent.BP_BuffComponent_C"))
  (Utilities|IsValid _returnvalue
    (:Is%20Valid
      (return (or (Default|IsInfiniteAmmo _returnvalue) (and (> (Variables|Default|GetAmmo) 0) (not (Default|IsInvincible _returnvalue))))))
    (:Is%20Not%20Valid
      (return (> (Variables|Default|GetAmmo) 0)))))

(fn EventAttachtoChar
  (params (Character :type Character%20Object%20Reference))
  (bind _output_get (Variables|Default|SetCharacter Character))
  (Physics|SetSimulatePhysics (Variables|Default|GetWeapon) false)
  (EventDispatchers|BindEventtoOnMontageEnded (Components|SkeletalMesh|GetAnimInstance (Variables|/Script/Engine.Character|GetMesh _output_get)) (EventDispatchers|CreateEvent :!event EventMontageEnd))
  (bind _returnvalue (Transformation|AttachComponentToComponent (Variables|/Script/Engine.Character|GetMesh _output_get) "weapon" "SnapToTarget" "SnapToTarget" "KeepWorld" true))
  (CallFunction|UpdateAmmoUI (Variables|Default|GetAmmo))
  (return _returnvalue))

(fn EventDetachfromChar
  (params (Character :type Character%20Object%20Reference))
  (Transformation|DetachFromComponent (Variables|Default|GetWeapon) "KeepWorld" "KeepWorld" "KeepWorld" true)
  (Physics|SetSimulatePhysics (Variables|Default|GetWeapon) true)
  (bind _character (Variables|Default|GetCharacter)
    (:then
      (EventDispatchers|UnbindEventfromOnMontageEnded (Components|SkeletalMesh|GetAnimInstance (Variables|/Script/Engine.Character|GetMesh _character)) (EventDispatchers|CreateEvent :!event EventMontageEnd))
      (CallFunction|UpdateAmmoUI)
      (Variables|Default|SetCharacter 0)
      (return true))
    (:else)))

(fn EventDoReload
  (bind _character (Variables|Default|GetCharacter)
    (:then
      (Animation|PlayAnimMontage _character (.reloadmontage (Variables|Default|GetWeaponData)) 1.0 "None"))
    (:else)))

(fn EventFire
  (bind _returnvalue (Game|GetPlayerCameraManager 0))
  (bind _returnvalue_2 (Transformation|GetActorLocation _returnvalue))
  (CallFunction|DoFireEffect)
  (if (== (Pawn|GetController (Variables|Default|GetCharacter)) (Game|GetPlayerController 0))
    ;[0.15 0.15 0.15 0.5] Client
    (CallFunction|ReqFire _returnvalue_2 (+ _returnvalue_2 (* (Transformation|GetActorForwardVector _returnvalue) 1e+05)))
    (return false)))

(fn EventReloadComplete
  (Utilities|IsOwnChar
    (:True
      (CallFunction|ReqReload)
      (return false))))

(fn EventTrigger
  (params (IsPress :type Boolean))
  (if IsPress
    (CallFunction|DoTrigger)
    (return false)))

(fn IsCanShoot
  (return (CallFunction|CanShoot)))

(fn IsReloading
  (bind _character (Variables|Default|GetCharacter)
    (:then
      (return (== (.reloadmontage (Variables|Default|GetWeaponData)) (Animation|Montage|GetCurrentActiveMontage (Components|SkeletalMesh|GetAnimInstance (Variables|/Script/Engine.Character|GetMesh _character))))))
    (:else)))